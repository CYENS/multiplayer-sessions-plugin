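; BP_MenuSetup is an actor that bootstraps the multiplayer session menu in a level.
; On BeginPlay it creates WBP_Menu, stores it and passes it the lobby and session maps through MenuSetup.
; Pressing Enter calls StartMultiplayerSession on the menu, or prints an on-screen warning if the menu is not valid.
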(event `self.ReceiveBeginPlay`
  (bind _returnvalue (`|CreateWidget` "/MultiplayerSessions/UI/WBP_Menu.WBP_Menu_C"))
  (bind _output_get (set `self.Menu` _returnvalue))
  (`Menu.MenuSetup` _output_get 4 "FreeForAll" (`self.Lobby Map`) (`self.Session Map`)))

(event `Key|Enter`
  (params (Key :type "Key Structure"))
  (:`Pressed`
    (`/Engine/EditorBlueprintResources/StandardMacros.IsValid` (`self.Menu`)
      (:`Is Valid`
        (`Menu.StartMultiplayerSession` (`self.Menu`)))
      (:`Is Not Valid`
        (`KismetSystemLibrary.PrintString` "Please make sure that Menu is initialised  " true true (struct :`R` 1.0 :`G` 0.041622 :`A` 1.0) 5.0)))))

(fn `UserConstructionScript`)